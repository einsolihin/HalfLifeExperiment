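; GM_HalfLife is a game mode Blueprint that runs a match countdown and shows game over when time runs out.
; BeginPlay creates the GameUI widget with its game-over panel hidden and leaves GameStart false.
; Once GameStart is true, a Delay on Tick paces one-second decrements of Minute and Second, which TimerFunction formats for the UI text.
; At zero it swaps panels, shows the cursor and switches to UI-only input.
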(event EventBeginPlay
  (bind _returnvalue (UserInterface|CreateWidget "/Game/GameUI.GameUI_C" (Game|GetPlayerController 0)))
  (Variables|Default|SetGameUI _returnvalue)
  (UserInterface|Viewport|AddtoViewport _returnvalue 0)
  (Widget|SetVisibility (Variables|/Game/GameUI.GameUI_C|GetGameOverPanel _returnvalue) "Hidden")
  (Variables|Default|SetGameStart false))

(event EventTick
  (params (DeltaSeconds :type Float%20%28single-precision%29))
  (bind _returnvalue (Game|GetPlayerController 0))
  (bind _gameui (Variables|Default|GetGameUI))
  (if (Variables|Default|GetGameStart)
    (Utilities|FlowControl|Delay 1.0)
    (if (== (Variables|Default|GetSecond) 0)
      (if (== (Variables|Default|GetMinute) 0)
        (Widget|SetVisibility (Variables|/Game/GameUI.GameUI_C|GetGameOverPanel _gameui) "Visible")
        (Widget|SetVisibility (Variables|/Game/GameUI.GameUI_C|GetGamePlayPanel _gameui) "Hidden")
        (Variables|/Script/Engine.PlayerController|SetbShowMouseCursor _returnvalue true)
        (Input|SetInputModeUIOnly _returnvalue (Variables|Default|GetGameUI) "DoNotLock")
        (else
          (Variables|Default|SetSecond 59)
          (bind _result (Math|Integer|DecrementInt (Variables|Default|GetMinute))
            (:%20%20
              (Variables|Default|SetMinute _result)
              (bind _timertext (CallFunction|TimerFunction (Variables|Default|GetSecond) (Variables|Default|GetMinute) :!label _label))
              (Variables|/Game/GameUI.GameUI_C|SetTimerText (Variables|Default|GetGameUI) _timertext)))))
      (else
        (bind _result_2 (Math|Integer|DecrementInt (Variables|Default|GetSecond))
          (:%20%20
            (Variables|Default|SetSecond _result_2)
            (goto _label)))))))

(fn ConstructionScript)

(fn TimerFunction
  (params (Second :type Integer) (Minute :type Integer))
  (return (Utilities|Text|ToText(String) (Utilities|String|Append (Utilities|String|ToString(Integer) Minute) " : " (Utilities|String|ToString(Integer) Second)))))